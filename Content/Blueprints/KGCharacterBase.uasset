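; KGCharacterBase is the shared knight character for players and enemies, handling combat, health and death.
; On begin play it attaches a sword, links its health-bar widget and binds a victory dance to game end.
; Montages drive chained melee, magic and flinches, which block new attacks and vary with attack state.
; Death ends the game for players and destroys AI knights, while construction tints hair through a dynamic material.
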(event Custom|LaunchMagicProjectile
  ;[1 1 1] Magic Attack
  (Game|SpawnActorfromClass "/Game/Blueprints/KG_ProjectileBase.KG_ProjectileBase_C" (Transformation|GetWorldTransform (Variables|Default|GetArrow1)) "Undefined" 0 self))

(event Custom|TryMelee
  (bind _mesh (Variables|Character|GetMesh))
  (bind _returnvalue (Components|SkeletalMesh|GetAnimInstance _mesh))
  (bind _returnvalue_2 (Animation|Montage|MontageGetCurrentSection _returnvalue "/Game/Assets/Knight/Anim_Montages/KnightAttackMontage.KnightAttackMontage"))
  ;[1 1 1] Melee Attack
  ;[1 1 1] Can attack only if NOT flinching.
  (if (not (Variables|Default|GetIsFlinching))
    (if (Class|AnimInstance|MontageIsActive _returnvalue "/Game/Assets/Knight/Anim_Montages/KnightAttackMontage.KnightAttackMontage")
      (switch name _returnvalue_2
        (:Attack1
          (Class|AnimInstance|MontageSetNextSection _returnvalue _returnvalue_2 "Attack2" "/Game/Assets/Knight/Anim_Montages/KnightAttackMontage.KnightAttackMontage")))
      (else
        (Animation|PlayAnimMontage "/Game/Assets/Knight/Anim_Montages/KnightAttackMontage.KnightAttackMontage" 1.0 "Attack1")))))

(event Custom|TryMagic
  ;[1 1 1] Magic Attack
  (if (not (Variables|Default|GetIsFlinching))
    (Animation|PlayAnimMontage "/Game/Assets/Knight/Anim_Montages/MagicShoot.MagicShoot" 1.0 "None")))

(event Custom|CreateSword
  ;[1 1 1] Add sword model to character's hand.
  (bind _returnvalue (Game|SpawnActorfromClass "/Game/Blueprints/BaseSword.BaseSword_C" (Transformation|GetActorTransform) "Undefined" 0 0))
  (Transformation|AttachComponentToComponent _returnvalue (Variables|Character|GetMesh) "Sword" "SnapToTarget" "SnapToTarget" "SnapToTarget" true)
  (Variables|Default|SetWeapon _returnvalue))

(event Custom|UsePrimaryAttack
  ;[1 1 1] Primary attack for enemies.
  (CallFunction|TryMelee))

(event Custom|EndGameDance
  ;[1 1 1] victory dance if game is done.
  (if (> (Variables|Default|Gethealth) 0.0)
    (Pawn|Components|CharacterMovement|DisableMovement (Variables|Character|GetCharacterMovement))
    (Animation|PlayAnimMontage "/Game/Assets/Knight/Anim_Montages/Victory_Montage.Victory_Montage" 1.0 "None")))

(event EventBeginPlay
  (CallFunction|CreateSword)
  ;[1 1 1] victory dance if game is done.
  (bind _askggame_mode (Utilities|Casting|CastToKGGameMode (Game|GetGameMode)))
  (EventDispatchers|BindEventtoEndGameDispatcher _askggame_mode (delegate Custom|EndGameDance))
  ;[1 1 1] Set UI health bar.
  (bind _asuihealth_bar (Utilities|Casting|CastToUIHealthBar (UserInterface|GetUserWidgetObject (Variables|Default|GetHealthBar))))
  (Default|SetOwningKnightCharacter _asuihealth_bar self))

(event Collision|EventActorBeginOverlap
  (params (OtherActor :type Actor%20Object%20Reference)))

(event EventTick
  (params (DeltaSeconds :type Float%20%28single-precision%29)))

(event Game|Damage|EventAnyDamage
  (params (Damage :type Float%20%28single-precision%29) (DamageType :type Damage%20Type%20Object%20Reference) (InstigatedBy :type Controller%20Object%20Reference) (DamageCauser :type Actor%20Object%20Reference))
  (bind _mesh (Variables|Character|GetMesh))
  (bind _returnvalue (Components|SkeletalMesh|GetAnimInstance _mesh))
  ;[1 1 1] set health upon damage
  (bind _output_get (Variables|Default|Sethealth (- (Variables|Default|Gethealth) Damage)))
  (if (<= _output_get 0.0)
    (Utilities|FlowControl|DoOnce false
      (:Completed
        (Variables|Default|SetIsFlinching true)
        (Pawn|Components|CharacterMovement|DisableMovement (Variables|Character|GetCharacterMovement))
        (bind _returnvalue_2 (Animation|PlayAnimMontage "/Game/Assets/Knight/Anim_Montages/PlayerDeath.PlayerDeath" 1.0 "None"))
        (if (Class|Controller|IsPlayerController (Pawn|GetController))
          (Default|EndGame (.AsKGGame%20Mode (Utilities|Casting|CastToKGGameMode (Game|GetGameMode))))
          (else
            (Utilities|FlowControl|Delay _returnvalue_2)
            (Actor|DestroyActor (Variables|Default|GetWeapon))
            (Actor|DestroyActor)))))
    (else
      (Variables|Default|SetIsFlinching true) ; Flinching if taking damage.
      ;[1 1 1] Large flinch if not in process of attacking.  Small flinch if in process of attacking.
      (if (Class|AnimInstance|MontageIsActive _returnvalue "/Game/Assets/Knight/Anim_Montages/KnightAttackMontage.KnightAttackMontage")
        (if (Utilities|Array|ContainsItem (Variables|Default|GetAttackMoves) (Animation|Montage|MontageGetCurrentSection _returnvalue "/Game/Assets/Knight/Anim_Montages/KnightAttackMontage.KnightAttackMontage"))
          (Variables|Default|SetIsFlinching false)
          (else
            (bind _returnvalue_3 (Animation|PlayAnimMontage "/Game/Assets/Knight/Anim_Montages/PlayerFinch.PlayerFinch" 1.0 "FlinchBig"))
            ;;[1 1 1] Stop flinching after flinching for a while.
            (Utilities|FlowControl|Delay _returnvalue_3)
            (Variables|Default|SetIsFlinching false)))
        (else
          (bind _returnvalue_4 (Animation|PlayAnimMontage "/Game/Assets/Knight/Anim_Montages/PlayerFinch.PlayerFinch" 1.0 "FlinchSmall"))
          (Utilities|FlowControl|Delay _returnvalue_4)
          (Variables|Default|SetIsFlinching false))))))

(fn ConstructionScript
  ;[1 1 1] Set hair color based on variable
  (bind _returnvalue (Rendering|Material|CreateDynamicMaterialInstance (Variables|Character|GetMesh) 0 0 "None" :!class /Script/Engine.PrimitiveComponent))
  (Rendering|Material|SetVectorParameterValue _returnvalue "HairColor" (Variables|Default|GetHairColor) :!class /Script/Engine.MaterialInstanceDynamic))
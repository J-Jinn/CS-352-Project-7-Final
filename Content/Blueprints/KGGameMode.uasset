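; Game mode that runs enemy waves and ends the match once the last wave is cleared.
; Each wave's class list is shuffled into a queue, which a one-second looping timer drains by spawning AI at random PlayerStarts.
; Enemy destruction advances the wave when the queue and KGAIControllerBase actors are both gone.
; Game end fires a dispatcher, blends to a random CameraActor, then restarts the level after a delay.
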(event Custom|SpawnEnemy
  ;[1 1 1] Spawn enemies.
  ;;[1 1 1] Spawn enemies if any in queue.
  (if (> (Utilities|Array|Length (Variables|Default|GetQueue)) 0)
    ;;[1 1 1] Spawn random # of enemies.
    (bind _outactors (Actor|GetAllActorsOfClass "/Script/Engine.PlayerStart"))
    (bind _returnvalue (AI|SpawnAIFromClass (Utilities|Array|Get(acopy) (Variables|Default|GetQueue)) 0 (Transformation|GetActorLocation (Utilities|Array|Get(acopy) _outactors (Math|Random|RandomInteger (Utilities|Array|Length _outactors)))) (Transformation|GetActorRotation (Utilities|Array|Get(acopy) _outactors (Math|Random|RandomInteger (Utilities|Array|Length _outactors)))) false))
    ;;[1 1 1] Remove from queue once spawned.
    (Utilities|Array|RemoveIndex (Variables|Default|GetQueue))
    ;;[1 1 1] Check wave is complete, every time a enemy is destroyed.
    (Game|BindEventtoOnDestroyed _returnvalue (delegate Custom|CheckWaveComplete))))

(event Custom|StartNewWave
  ;[1 1 1] Spawn enemies.
  ;;[1 1 1] Spawn randomized waves based on queue.
  (Math|Integer|IncrementInt (Variables|Default|GetWaveIndex)
    (:%20%20
      (Default|CallNewWave)
      ;;;[1 1 1] if not the last wave.
      (if (< (Utilities|Array|LastIndex (Variables|Default|GetWaves)) (Variables|Default|GetWaveIndex))
        (CallFunction|EndGame)
        (else
          (bind _output_get (Variables|Default|SetQueue (.classtospawn (Utilities|Array|Get(acopy) (Variables|Default|GetWaves) (Variables|Default|GetWaveIndex)))))
          (Utilities|Array|Shuffle _output_get))))))

(event Custom|EndGame
  ;[1 1 1] play victory dance and restart level
  (Default|CallEndGameDispatcher)
  (bind _outactors (Actor|GetAllActorsOfClass "/Script/Engine.CameraActor"))
  (Game|Player|SetViewTargetwithBlend (Game|GetPlayerController 0) (Utilities|Array|Get(acopy) _outactors (Math|Random|RandomInteger (Utilities|Array|Length _outactors))) 4.0 "VTBlend_Linear" 0.0 true)
  (Utilities|FlowControl|Delay 6.0)
  (Development|ExecuteConsoleCommand "restartlevel" 0))

(event Custom|CheckWaveComplete
  (params (DestroyedActor :type Actor%20Object%20Reference))
  ;[1 1 1] Spawn enemies.
  ;;[1 1 1] Check wave is complete, every time a enemy is destroyed.
  (if (== (Utilities|Array|Length (Variables|Default|GetQueue)) 0)
    ;;[1 1 1] If no enemies left, start new wave.
    (bind _outactors (Actor|GetAllActorsOfClass "/Game/Blueprints/KGAIControllerBase.KGAIControllerBase_C"))
    (if (== (Utilities|Array|Length _outactors) 0)
      (CallFunction|StartNewWave))))

(event Custom|ResetGAme
  ;[1 1 1] Spawn enemies.
  ;;[1 1 1] Spawn randomized waves based on queue.
  ;;;[1 1 1] so we don't skip wave 0.
  (Variables|Default|SetWaveIndex 0)
  (bind _output_get (Variables|Default|SetQueue (.classtospawn (Utilities|Array|Get(acopy) (Variables|Default|GetWaves) (Variables|Default|GetWaveIndex)))))
  (Utilities|Array|Shuffle _output_get))

(event EventBeginPlay
  ;[1 1 1] Spawn enemies.
  (Utilities|Time|SetTimerbyEvent (delegate Custom|SpawnEnemy) 1.0 true)
  (CallFunction|ResetGAme))

(event EventTick
  (params (DeltaSeconds :type Float%20%28single-precision%29)))

(fn ConstructionScript)
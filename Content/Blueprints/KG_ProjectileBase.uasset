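; Base magic projectile that damages KG characters on contact and leaves a small area blast when destroyed.
; Overlapping a KGCharacterBase other than its Instigator applies direct damage and destroys the projectile, while other overlaps are ignored.
; The Destroyed event spawns an impulse particle effect and applies radial damage credited to the Instigator's controller, so the blast follows any destruction, not just a hit.
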(event EventBeginPlay)

(event Collision|EventActorBeginOverlap
  (params (OtherActor :type Actor%20Object%20Reference))
  (bind _instigator (Variables|Actor|GetInstigator))
  ;[1 1 1] Magic only hits target, not self.
  (bind _askgcharacter_base (Utilities|Casting|CastToKGCharacterBase OtherActor))
  (if (not (== _askgcharacter_base _instigator))
    (Game|Damage|ApplyDamage _askgcharacter_base 5e+01 (Pawn|GetController _instigator) self)
    (Actor|DestroyActor)))

(event EventTick
  (params (DeltaSeconds :type Float%20%28single-precision%29)))

(event EventDestroyed
  ;[1 1 1] Magic effect will disappear after time and AOE damage.
  (Effects|SpawnEmitteratLocation "/Game/Assets/Effects/P_Impulse.P_Impulse" (Transformation|GetActorLocation))
  (Game|Damage|ApplyRadialDamage 2e+01 (Transformation|GetActorLocation) 5e+01 0 0 self (Pawn|GetController (Variables|Actor|GetInstigator)) false "ECC_Visibility"))

(fn ConstructionScript)